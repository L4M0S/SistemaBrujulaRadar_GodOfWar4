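; Compass-style radar component that shows world directions and mission markers with distances on a HUD widget.
; InicializarRadar creates WB_Principal and fills its radar widget from the direction and default marker arrays.
; Player turn and move events refresh it while visible, mapping shortest yaw delta over camera FOV to horizontal offset and hiding out-of-range entries.
; Marker distances ignore height, and visibility changes can play a locked, reversible fade animation.
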(event `InicializarRadar`
  (params (Jugador :type "Actor Object Reference") (Camara :type "CameraComponent Object Reference"))
  ;[1 1 1] Inicializar Radar
  (set `self.JugadorReferencia` Jugador)
  (set `self.ReferenciaCamara` Camara)
  (bind _returnvalue (`|CreateWidget` "/Game/SistemaDeRadar/Widgets/WB_Principal.WB_Principal_C"))
  (bind _output_get (set `self.WidgetPrincipalReferencia` _returnvalue))
  (set `self.WidgetRadarReferencia` (`/Game/SistemaDeRadar/Widgets/WB_Principal.Radar_Widget` _output_get))
  (for _array_element (`self.Direcciones`)
    (`/Game/SistemaDeRadar/Widgets/WB_Radar.AnadirDireccion` (`self.WidgetRadarReferencia`) _array_element))
  (for _array_element_2 (`self.MisionMarcadorPredeterminado`)
    (`self.AnadirMarcadorAlRadar` _array_element_2))
  (`self.ActualizarDistanciaMarcador`)
  (`self.ActualzarPosicionMarcadores`)
  (`self.ActualizarWidgetsDireccion`)
  (`UserWidget.AddToViewport` (`self.WidgetPrincipalReferencia`) 0))

(event `AjustarVisibilidad`
  (params (`Visible?` :type Boolean) (`Animar?` :type Boolean))
  (bind _widgetradarreferencia (`self.WidgetRadarReferencia`))
  (bind _blendout (`/Game/SistemaDeRadar/Widgets/WB_Radar.BlendOut` _widgetradarreferencia))
  (bind _blendout_2 (`/Game/SistemaDeRadar/Widgets/WB_Radar.BlendOut` _widgetradarreferencia))
  ;[1 1 1] Ajustar Visibilidad del Radar (Visible u Oculto)
  (if (and (!= `Visible?` (`self.Visible?`)) (`self.PuedeCambiarVisibilidad?`))
    (set `self.PuedeCambiarVisibilidad?` false)
    (set `self.Visible?` `Visible?`)
    (if `Animar?`
      (if (`self.Visible?`)
        (`Widget.SetVisibility` _widgetradarreferencia "SelfHitTestInvisible")
        (`UserWidget.PlayAnimation` _widgetradarreferencia _blendout_2 0.0 1 "Reverse" 1.0)
        (`KismetSystemLibrary.Delay` (`WidgetAnimation.GetEndTime` _blendout_2))
        (set `self.PuedeCambiarVisibilidad?` true)
        (else
          (`UserWidget.PlayAnimation` _widgetradarreferencia _blendout 0.0 1 "Forward" 1.0)
          (`KismetSystemLibrary.Delay` (`WidgetAnimation.GetEndTime` _blendout))
          (`Widget.SetVisibility` (`self.WidgetRadarReferencia`) "Hidden")
          (set `self.PuedeCambiarVisibilidad?` true)))
      (else
        (`Widget.SetVisibility` (`self.WidgetRadarReferencia`) (select `bool` (`self.Visible?`) :`false` "Hidden" :`true` "SelfHitTestInvisible" :!type "ESlateVisibility Enum"))
        (set `self.PuedeCambiarVisibilidad?` true)))))

(event `JugadorGirando`
  ;[1 1 1] Jugador Girando
  (if (`self.Visible?`)
    (`self.ActualizarWidgetsDireccion`)
    (`self.ActualzarPosicionMarcadores`)))

(event `JugadorMoviendose`
  ;[1 1 1] Jugador Moviendose
  (if (`self.Visible?`)
    (`self.ActualizarDistanciaMarcador`)
    (`self.ActualzarPosicionMarcadores`)))

(fn `ActualizarDistanciaMarcador`
  (for (_array_element _array_index) (`/Game/SistemaDeRadar/Widgets/WB_Radar.WidgetMarcador` (`self.WidgetRadarReferencia`))
    (`/Game/SistemaDeRadar/Widgets/WB_Marcador.ActualizarDistancia` _array_element (`KismetMathLibrary.Round` (/ (`KismetMathLibrary.VSize` (- (`KismetMathLibrary.MakeVector` (.x (`.Ubicacion_5_54F27275466EF2D118C33F8277D165E5` (break `/Game/SistemaDeRadar/Estructuras/S_MarcadorInfo` (`|GetArrayItem` (`self.MisionMarcadores`) _array_index)))) (.y (`.Ubicacion_5_54F27275466EF2D118C33F8277D165E5` (break `/Game/SistemaDeRadar/Estructuras/S_MarcadorInfo` (`|GetArrayItem` (`self.MisionMarcadores`) _array_index)))) 0.0) (`KismetMathLibrary.MakeVector` (.x (`Actor.K2_GetActorLocation` (`self.JugadorReferencia`))) (.y (`Actor.K2_GetActorLocation` (`self.JugadorReferencia`)))))) (`self.UnidadesPorMetro`)))))
  (return))

(fn `ActualizarWidgetsDireccion`
  (for (_array_element _array_index) (`/Game/SistemaDeRadar/Widgets/WB_Radar.WidgetDireccion` (`self.WidgetRadarReferencia`))
    (bind (_traslacion _sentidoagujasreloj_ _envistadelradar_) (`self.RotacionToTraslacion` (`SceneComponent.K2_GetComponentRotation` (`self.ReferenciaCamara`)) (`KismetMathLibrary.MakeRotator` 0.0 0.0 (`KismetMathLibrary.Conv_IntToDouble` (`.RotacionMundo_5_B5FD052440DD57D45D4C09B363ACDA44` (break `/Game/SistemaDeRadar/Estructuras/S_DireccionesInfo` (`|GetArrayItem` (`self.Direcciones`) _array_index)))))))
    (if _envistadelradar_
      (`Widget.SetRenderTranslation` _array_element _traslacion)
      (bind _returnvalue (`Widget.IsVisible` _array_element))
      (if (not _returnvalue)
        (`Widget.SetVisibility` _array_element "SelfHitTestInvisible"))
      (elif _returnvalue
        (`Widget.SetVisibility` _array_element "Hidden")))))

(fn `ActualzarPosicionMarcadores`
  (for (_array_element _array_index) (`/Game/SistemaDeRadar/Widgets/WB_Radar.WidgetMarcador` (`self.WidgetRadarReferencia`))
    (bind (_traslacion _sentidoagujasreloj_ _envistadelradar_) (`self.RotacionToTraslacion` (`SceneComponent.K2_GetComponentRotation` (`self.ReferenciaCamara`)) (`KismetMathLibrary.FindLookAtRotation` (`Actor.K2_GetActorLocation` (`self.JugadorReferencia`)) (`.Ubicacion_5_54F27275466EF2D118C33F8277D165E5` (break `/Game/SistemaDeRadar/Estructuras/S_MarcadorInfo` (`|GetArrayItem` (`self.MisionMarcadores`) _array_index))))))
    (if _envistadelradar_
      (`Widget.SetRenderTranslation` _array_element _traslacion)
      (bind _returnvalue (`Widget.IsVisible` _array_element))
      (if (not _returnvalue)
        (`Widget.SetVisibility` _array_element "SelfHitTestInvisible"))
      (elif _returnvalue
        (`Widget.SetVisibility` _array_element "Hidden"))))
  (return))

(fn `AnadirMarcadorAlRadar`
  (params (Infomacion :type "/Game/SistemaDeRadar/Estructuras/S_MarcadorInfo Structure"))
  (locals (LocalInfo :type "/Game/SistemaDeRadar/Estructuras/S_MarcadorInfo Structure"))
  (bind _widgetradarreferencia (`self.WidgetRadarReferencia`))
  (bind _output_get (set `local.LocalInfo` Infomacion))
  (`KismetArrayLibrary.Array_Add` (`self.MisionMarcadores`) _output_get)
  (`/Engine/EditorBlueprintResources/StandardMacros.IsValid` _widgetradarreferencia
    (:`Is Valid`
      (`/Game/SistemaDeRadar/Widgets/WB_Radar.AnadirMarcador` _widgetradarreferencia (`.Tipo_2_6413CF8B481E15A9C0BE31843FC93B67` (break `/Game/SistemaDeRadar/Estructuras/S_MarcadorInfo` (`local.LocalInfo`))))
      (return))
    (:`Is Not Valid`
      (return))))

(fn `IntercambiarVisibilidad`
  (params (`Animar?` :type Boolean))
  (`self.AjustarVisibilidad` (not (`self.Visible?`)) `Animar?`)
  (return))

(fn `ObtenerDeltaSentidoAgujasReloj`
  (params (A :type "Float (double-precision)") (B :type "Float (double-precision)") (`SentidoAgujasReloj?` :type Boolean))
  (returns (Delta :type "Float (double-precision)"))
  (bind _returnvalue (mod B 360.0))
  (bind _returnvalue_2 (mod A 360.0))
  (bind _returnvalue_3 (mod A 360.0))
  (bind _returnvalue_4 (mod B 360.0))
  (if `SentidoAgujasReloj?`
    (`/Engine/EditorBlueprintResources/StandardMacros.CompareFloat` _returnvalue_3 _returnvalue_4
      (:`>`
        (return (- 360.0 (- _returnvalue_3 _returnvalue_4))))
      (:`==`
        (return 0.0))
      (:`<`
        (return (- _returnvalue_4 _returnvalue_3))))
    (else
      (`/Engine/EditorBlueprintResources/StandardMacros.CompareFloat` _returnvalue_2 _returnvalue
        (:`>`
          (return (- _returnvalue_2 _returnvalue)))
        (:`==`
          (return 0.0))
        (:`<`
          (return (- 360.0 (- _returnvalue_2 _returnvalue))))))))

(fn `RotacionToGrados`
  (params (InRotacion :type "Float (double-precision)"))
  (returns (OutGrados :type "Float (double-precision)"))
  (return (`KismetMathLibrary.SelectFloat` (mod (+ InRotacion 360.0) 360.0) InRotacion (< InRotacion 0.0))))

(fn `RotacionToTraslacion`
  (params (RotacionA :type "Rotator Structure") (RotacionB :type "Rotator Structure"))
  (returns (Traslacion :type "Vector2D Structure") (`SentidoAgujasReloj?` :type Boolean) (`EnVistaDelRadar?` :type Boolean))
  (bind _maxwidgettraslacion (`self.MaxWidgetTraslacion`))
  (bind _outgrados (`self.RotacionToGrados` (.yaw RotacionA)))
  (bind _outgrados_2 (`self.RotacionToGrados` (.yaw RotacionB)))
  (bind _fieldofview (`CameraComponent.FieldOfView` (`self.ReferenciaCamara`)))
  (bind _delta (`self.ObtenerDeltaSentidoAgujasReloj` _outgrados _outgrados_2))
  (bind _delta_2 (`self.ObtenerDeltaSentidoAgujasReloj` _outgrados _outgrados_2 true))
  (bind _returnvalue (/ _delta_2 _fieldofview))
  (bind _returnvalue_2 (/ _delta _fieldofview))
  (`/Engine/EditorBlueprintResources/StandardMacros.CompareFloat` _delta_2 _delta
    (:`>`
      (if (<= _returnvalue_2 1.0)
        (return (`KismetMathLibrary.MakeVector2D` (* (`KismetMathLibrary.Lerp` 0.0 _maxwidgettraslacion _returnvalue_2) -1.0)) false true)
        (else
          (return (0.0 0.0) false false))))
    (:`==`
      _)
    (:`<`
      _))
  (if (<= _returnvalue 1.0)
    (return (`KismetMathLibrary.MakeVector2D` (`KismetMathLibrary.Lerp` 0.0 _maxwidgettraslacion _returnvalue)) true true)
    (else
      (return (0.0 0.0) true false))))