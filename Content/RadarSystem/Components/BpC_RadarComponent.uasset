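; Radar component that drives a compass-style bar showing directions, quest markers, landmarks and monsters relative to the player's camera.
; InitializeRadar creates the main widget and fills it; player turn and move events, plus monster moves, refresh positions, distances and quest elevation arrows.
; Yaw deltas against camera FOV become horizontal offsets, hiding out-of-view icons or optionally pinning quest markers to the edges.
; Nearby secrets highlight the bar, and visibility toggles can animate.
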(event `InitializeRadar`
  (params (Player :type "Actor Object Reference") (Camera :type "CameraComponent Object Reference"))
  (set `self.PlayerReference` Player)
  (set `self.CameraReference` Camera)
  (bind _returnvalue (`|CreateWidget` "/Game/RadarSystem/Widgets/W_Main.W_Main_C"))
  (bind _output_get (set `self.MainWidgetReference` _returnvalue))
  (set `self.RadarWidgetReference` (`/Game/RadarSystem/Widgets/W_Main.RadarWidget` _output_get))
  (for _array_element (`self.Directions`)
    (`/Game/RadarSystem/Widgets/W_Radar.AddDirection` (`self.RadarWidgetReference`) _array_element))
  (for _array_element_2 (`self.DefaultQuestMarkers`)
    (`self.AddMarkerToRadar` _array_element_2))
  (bind _outactors (`GameplayStatics.GetAllActorsOfClass` "/Game/RadarSystem/Classes/Bp_Master_Landmark.Bp_Master_Landmark_C"))
  (for _array_element_3 _outactors
    (`self.AddLandmarkToRadar` _array_element_3))
  (`self.OnBecomeVisible`)
  (`self.OnRadarInitialized`)
  (`UserWidget.AddToViewport` (`self.MainWidgetReference`) 0))

(event `OnPlayerTurned`
  (if (`self.Visible?`)
    (`self.UpdateDirectionWidgets`)
    (`self.UpdateMarkerPositions`)
    (`self.UpdateLandmarkPositions`)
    (`self.UpdateMonsterMarkerPositions`)))

(event `OnPlayerMoved`
  (if (`self.Visible?`)
    (`self.UpdateMarkerDistances`)
    (`self.UpdateMarkerPositions`)
    (`self.UpdateLandmarkPositions`)
    (`self.UpdateMonsterMarkerDistances`)
    (`self.UpdateMonsterMarkerPositions`)
    (`self.UpdateMarkerElevations`)))

(event `OnEnterSecretRange`
  (params (Secret :type "/Game/RadarSystem/Classes/Bp_Master_Secret Object Reference"))
  (bind _secretsinrange (`self.SecretsInRange`))
  (if (not (`KismetArrayLibrary.Array_Contains` (`self.SecretsInRange`) Secret))
    (`KismetArrayLibrary.Array_Add` _secretsinrange Secret)
    (if (== (`KismetArrayLibrary.Array_Length` _secretsinrange) 1)
      (`/Game/RadarSystem/Widgets/W_Radar.HighlightRadar` (`self.RadarWidgetReference`) true))))

(event `OnRadarInitialized`
  (bind _outactors (`GameplayStatics.GetAllActorsOfClass` "/Game/RadarSystem/Classes/Bp_Master_Monster.Bp_Master_Monster_C"))
  (for _array_element _outactors
    (`/Game/RadarSystem/Classes/Bp_Master_Monster.OnRadarIntialized` _array_element)))

(event `OnMonsterMoved`
  (params (Monster :type "/Game/RadarSystem/Classes/Bp_Master_Monster Object Reference"))
  (`self.UpdateMarkerDistanceForMonster` Monster)
  (`self.UpdateMarkerPositionForMonster` Monster))

(event `OnLeaveSecretRange`
  (params (Secret :type "/Game/RadarSystem/Classes/Bp_Master_Secret Object Reference"))
  (bind _secretsinrange (`self.SecretsInRange`))
  (if (`KismetArrayLibrary.Array_Contains` (`self.SecretsInRange`) Secret)
    (`KismetArrayLibrary.Array_RemoveItem` _secretsinrange Secret)
    (if (== (`KismetArrayLibrary.Array_Length` _secretsinrange) 0)
      (`/Game/RadarSystem/Widgets/W_Radar.HighlightRadar` (`self.RadarWidgetReference`) false))))

(event `SetVisibility`
  (params (`Visible?` :type Boolean) (`Animate?` :type Boolean))
  (bind _radarwidgetreference (`self.RadarWidgetReference`))
  (bind _blendout (`/Game/RadarSystem/Widgets/W_Radar.BlendOut` _radarwidgetreference))
  (bind _blendout_2 (`/Game/RadarSystem/Widgets/W_Radar.BlendOut` _radarwidgetreference))
  (if (and (!= `Visible?` (`self.Visible?`)) (`self.CanChangeVisibility?`))
    (set `self.CanChangeVisibility?` false)
    (set `self.Visible?` `Visible?`)
    (if `Animate?`
      (if (`self.Visible?`)
        (`self.OnBecomeVisible`)
        (`Widget.SetVisibility` _radarwidgetreference "SelfHitTestInvisible")
        (`UserWidget.PlayAnimation` _radarwidgetreference _blendout 0.0 1 "Reverse" 1.0)
        (`KismetSystemLibrary.Delay` (`WidgetAnimation.GetEndTime` _blendout))
        (set `self.CanChangeVisibility?` true)
        (else
          (`UserWidget.PlayAnimation` _radarwidgetreference _blendout_2 0.0 1 "Forward" 1.0)
          (`KismetSystemLibrary.Delay` (`WidgetAnimation.GetEndTime` _blendout_2))
          (`Widget.SetVisibility` (`self.RadarWidgetReference`) "Hidden")
          (set `self.CanChangeVisibility?` true)))
      (else
        (if (`self.Visible?`)
          (`self.OnBecomeVisible`))
        (`Widget.SetVisibility` (`self.RadarWidgetReference`) (select `bool` (`self.Visible?`) :`false` "Hidden" :`true` "SelfHitTestInvisible" :!type "ESlateVisibility Enum"))
        (set `self.CanChangeVisibility?` true)))))

(event `OnBecomeVisible`
  (`self.UpdateDirectionWidgets`)
  (`self.UpdateMarkerDistances`)
  (`self.UpdateMarkerPositions`)
  (`self.UpdateLandmarkPositions`)
  (`self.UpdateMonsterMarkerDistances`)
  (`self.UpdateMonsterMarkerPositions`)
  (`self.UpdateMarkerElevations`))

(fn `AddLandmarkToRadar`
  (params (Landmark :type "/Game/RadarSystem/Classes/Bp_Master_Landmark Object Reference"))
  (bind _radarwidgetreference (`self.RadarWidgetReference`))
  (if (`KismetArrayLibrary.Array_Contains` (`self.Landmarks`) Landmark)
    (return)
    (else
      (`KismetArrayLibrary.Array_Add` (`self.Landmarks`) Landmark)
      (`/Engine/EditorBlueprintResources/StandardMacros.IsValid` _radarwidgetreference
        (:`Is Valid`
          (`/Game/RadarSystem/Widgets/W_Radar.AddLandmark` _radarwidgetreference (`/Game/RadarSystem/Classes/Bp_Master_Landmark.IconOnRadar` Landmark))
          (return))
        (:`Is Not Valid`
          (return))))))

(fn `AddMarkerToRadar`
  (params (Info :type "/Game/RadarSystem/Structures/S_MarkerInfo Structure"))
  (locals (localInfo :type "/Game/RadarSystem/Structures/S_MarkerInfo Structure"))
  (bind _radarwidgetreference (`self.RadarWidgetReference`))
  (bind _output_get (set `local.localInfo` Info))
  (`KismetArrayLibrary.Array_Add` (`self.QuestMarkers`) _output_get)
  (`/Engine/EditorBlueprintResources/StandardMacros.IsValid` _radarwidgetreference
    (:`Is Valid`
      (`/Game/RadarSystem/Widgets/W_Radar.AddMarker` _radarwidgetreference (`.Type_2_A92FE0E24594A3314A1D7194C4E47164` (break `/Game/RadarSystem/Structures/S_MarkerInfo` (`local.localInfo`))))
      (return))
    (:`Is Not Valid`
      (return))))

(fn `AddMonsterToRadar`
  (params (Monster :type "/Game/RadarSystem/Classes/Bp_Master_Monster Object Reference"))
  (returns (`Success?` :type Boolean))
  (`/Engine/EditorBlueprintResources/StandardMacros.IsValid` (`self.RadarWidgetReference`)
    (:`Is Valid`
      (if (not (`KismetArrayLibrary.Array_Contains` (`self.MonstersOnRadar`) Monster))
        (`KismetArrayLibrary.Array_Add` (`self.MonstersOnRadar`) Monster)
        (`/Game/RadarSystem/Widgets/W_Radar.AddMonsterMarker` (`self.RadarWidgetReference`))
        (`self.UpdateMarkerDistanceForMonster` Monster)
        (`self.UpdateMarkerPositionForMonster` Monster)
        (return true)
        (else
          _)))
    (:`Is Not Valid`
      _))
  (return false))

(fn `DistanceToPlayer`
  (params (Actor :type "Actor Object Reference"))
  (returns (Distance :type Integer))
  (return (`KismetMathLibrary.Round` (/ (`KismetMathLibrary.VSize` (- (`KismetMathLibrary.MakeVector` (.x (`Actor.K2_GetActorLocation` Actor)) (.y (`Actor.K2_GetActorLocation` Actor))) (`KismetMathLibrary.MakeVector` (.x (`Actor.K2_GetActorLocation` (`self.PlayerReference`))) (.y (`Actor.K2_GetActorLocation` (`self.PlayerReference`)))))) (`self.UnitsPerMeter`)))))

(fn `GetDeltaClockwise`
  (params (A :type "Float (double-precision)") (B :type "Float (double-precision)") (`Clockwise?` :type Boolean))
  (returns (Delta :type "Float (double-precision)"))
  (bind _returnvalue (mod B 360.0))
  (bind _returnvalue_2 (mod A 360.0))
  (bind _returnvalue_3 (mod A 360.0))
  (bind _returnvalue_4 (mod B 360.0))
  (if `Clockwise?`
    (`/Engine/EditorBlueprintResources/StandardMacros.CompareFloat` _returnvalue_3 _returnvalue_4
      (:`>`
        (return (- 360.0 (- _returnvalue_3 _returnvalue_4))))
      (:`==`
        (return 0.0))
      (:`<`
        (return (- _returnvalue_4 _returnvalue_3))))
    (else
      (`/Engine/EditorBlueprintResources/StandardMacros.CompareFloat` _returnvalue_2 _returnvalue
        (:`>`
          (return (- _returnvalue_2 _returnvalue)))
        (:`==`
          (return 0.0))
        (:`<`
          (return (- 360.0 (- _returnvalue _returnvalue_2))))))))

(fn `RemoveMarkerAtIndex`
  (params (Index :type Integer))
  (returns (`Success?` :type Boolean))
  (bind _questmarkers (`self.QuestMarkers`))
  (if (and (`KismetMathLibrary.InRange_IntInt` Index 0 (`KismetArrayLibrary.Array_LastIndex` _questmarkers)) (> (`KismetArrayLibrary.Array_Length` _questmarkers) 0))
    (bind _success_ (`self.RemoveQuestMarker` (`|GetArrayItem` (`self.QuestMarkers`) Index)))
    (return _success_)
    (else
      (return false))))

(fn `RemoveMonsterFromRadar`
  (params (Monster :type "/Game/RadarSystem/Classes/Bp_Master_Monster Object Reference"))
  (locals (localIndex :type Integer :default 0))
  (bind _localindex (`local.localIndex`))
  (bind _returnvalue (`KismetArrayLibrary.Array_Find` (`self.MonstersOnRadar`) Monster))
  (bind _monstermarkerwidgets (`/Game/RadarSystem/Widgets/W_Radar.MonsterMarkerWidgets` (`self.RadarWidgetReference`)))
  (bind _output (`|GetArrayItem` _monstermarkerwidgets (`local.localIndex`)))
  (if (>= _returnvalue 0)
    (set `local.localIndex` _returnvalue)
    (`KismetArrayLibrary.Array_Remove` (`self.MonstersOnRadar`) _localindex)
    (`/Engine/EditorBlueprintResources/StandardMacros.IsValid` _output
      (:`Is Valid`
        (`Widget.RemoveFromParent` _output)
        (`KismetArrayLibrary.Array_Remove` _monstermarkerwidgets _localindex)
        (return))
      (:`Is Not Valid`
        (return)))
    (else
      (return))))

(fn `RemoveQuestMarker`
  (params (Marker :type "/Game/RadarSystem/Structures/S_MarkerInfo Structure"))
  (returns (`Success?` :type Boolean))
  (locals (localIndex :type Integer :default 0))
  (bind _localindex (`local.localIndex`))
  (bind _returnvalue (`KismetArrayLibrary.Array_Find` (`self.QuestMarkers`) Marker))
  (bind _markerwidgets (`/Game/RadarSystem/Widgets/W_Radar.MarkerWidgets` (`self.RadarWidgetReference`)))
  (if (>= _returnvalue 0)
    (set `local.localIndex` _returnvalue)
    (`KismetArrayLibrary.Array_Remove` (`self.QuestMarkers`) _localindex)
    (`Widget.RemoveFromParent` (`|GetArrayItem` _markerwidgets (`local.localIndex`)))
    (`KismetArrayLibrary.Array_Remove` _markerwidgets _localindex)
    (return true)
    (else
      (return false))))

(fn `RotationsToTranslation`
  (params (`Rotation A` :type "Rotator Structure") (`Rotation B` :type "Rotator Structure"))
  (returns (Translation :type "Vector2D Structure") (`Clockwise?` :type Boolean) (`InRadarSight?` :type Boolean))
  (bind _maxwidgettranslation (`self.MaxWidgetTranslation`))
  (bind _out (`self.RotationToCircleDegrees` (.yaw `Rotation B`)))
  (bind _out_2 (`self.RotationToCircleDegrees` (.yaw `Rotation A`)))
  (bind _fieldofview (`CameraComponent.FieldOfView` (`self.CameraReference`)))
  (bind _delta (`self.GetDeltaClockwise` _out_2 _out))
  (bind _delta_2 (`self.GetDeltaClockwise` _out_2 _out true))
  (bind _returnvalue (/ _delta _fieldofview))
  (bind _returnvalue_2 (/ _delta_2 _fieldofview))
  (`/Engine/EditorBlueprintResources/StandardMacros.CompareFloat` _delta_2 _delta
    (:`>`
      (if (<= _returnvalue 1.0)
        (return (`KismetMathLibrary.MakeVector2D` (* (`KismetMathLibrary.Lerp` 0.0 _maxwidgettranslation _returnvalue) -1.0)) false true)
        (else
          (return (0.0 0.0) false false))))
    (:`==`
      _)
    (:`<`
      _))
  (if (<= _returnvalue_2 1.0)
    (return (`KismetMathLibrary.MakeVector2D` (`KismetMathLibrary.Lerp` 0.0 _maxwidgettranslation _returnvalue_2)) true true)
    (else
      (return (0.0 0.0) true false))))

(fn `RotationToCircleDegrees`
  (params (In :type "Float (double-precision)"))
  (returns (Out :type "Float (double-precision)"))
  (return (`KismetMathLibrary.SelectFloat` (mod (+ In 360.0) 360.0) In (< In 0.0))))

(fn `ToggleVisibility`
  (params (`Animate?` :type Boolean))
  (`self.SetVisibility` (not (`self.Visible?`)) `Animate?`)
  (return))

(fn `UpdateDirectionWidgets`
  (for (_array_element _array_index) (`/Game/RadarSystem/Widgets/W_Radar.DirectionWidgets` (`self.RadarWidgetReference`))
    (bind (_translation _clockwise_ _inradarsight_) (`self.RotationsToTranslation` (`SceneComponent.K2_GetComponentRotation` (`self.CameraReference`)) (`KismetMathLibrary.MakeRotator` 0.0 0.0 (`KismetMathLibrary.Conv_IntToDouble` (`.WorldRotation_5_140EC7674DD29F844C10689F1D40CD83` (break `/Game/RadarSystem/Structures/S_DirectionInfo` (`|GetArrayItem` (`self.Directions`) _array_index)))))))
    (if _inradarsight_
      (`Widget.SetRenderTranslation` _array_element _translation)
      (bind _returnvalue (`Widget.IsVisible` _array_element))
      (if (not _returnvalue)
        (`Widget.SetVisibility` _array_element "SelfHitTestInvisible"))
      (elif _returnvalue
        (`Widget.SetVisibility` _array_element "Hidden"))))
  (return))

(fn `UpdateLandmarkPositions`
  (for (_array_element _array_index) (`/Game/RadarSystem/Widgets/W_Radar.LandmarkWidgets` (`self.RadarWidgetReference`))
    (bind (_translation _clockwise_ _inradarsight_) (`self.RotationsToTranslation` (`SceneComponent.K2_GetComponentRotation` (`self.CameraReference`)) (`KismetMathLibrary.FindLookAtRotation` (`Actor.K2_GetActorLocation` (`self.PlayerReference`)) (`Actor.K2_GetActorLocation` (`|GetArrayItem` (`self.Landmarks`) _array_index)))))
    (if _inradarsight_
      (`Widget.SetRenderTranslation` _array_element _translation)
      (bind _returnvalue (`Widget.IsVisible` _array_element))
      (if (not _returnvalue)
        (`Widget.SetVisibility` _array_element "SelfHitTestInvisible"))
      (elif _returnvalue
        (`Widget.SetVisibility` _array_element "Hidden"))))
  (return))

(fn `UpdateMarkerDistanceForMonster`
  (params (Monster :type "/Game/RadarSystem/Classes/Bp_Master_Monster Object Reference"))
  (locals (localIndex :type Integer :default 0))
  (bind _returnvalue (`KismetArrayLibrary.Array_Find` (`self.MonstersOnRadar`) Monster))
  (bind _output (`|GetArrayItem` (`/Game/RadarSystem/Widgets/W_Radar.MonsterMarkerWidgets` (`self.RadarWidgetReference`)) (`local.localIndex`)))
  (if (>= _returnvalue 0)
    (set `local.localIndex` _returnvalue)
    (`/Engine/EditorBlueprintResources/StandardMacros.IsValid` _output
      (:`Is Valid`
        (`/Game/RadarSystem/Widgets/W_MonsterMarker.UpdateDistance` _output (`self.DistanceToPlayer` Monster))))))

(fn `UpdateMarkerDistances`
  (for (_array_element _array_index) (`/Game/RadarSystem/Widgets/W_Radar.MarkerWidgets` (`self.RadarWidgetReference`))
    (`/Game/RadarSystem/Widgets/W_Marker.UpdateDistance` _array_element (`KismetMathLibrary.Round` (/ (`KismetMathLibrary.VSize` (- (`KismetMathLibrary.MakeVector` (.x (`.Location_5_DE6DBAFE464D624CFBEFE59C7B88E7BD` (break `/Game/RadarSystem/Structures/S_MarkerInfo` (`|GetArrayItem` (`self.QuestMarkers`) _array_index)))) (.y (`.Location_5_DE6DBAFE464D624CFBEFE59C7B88E7BD` (break `/Game/RadarSystem/Structures/S_MarkerInfo` (`|GetArrayItem` (`self.QuestMarkers`) _array_index))))) (`KismetMathLibrary.MakeVector` (.x (`Actor.K2_GetActorLocation` (`self.PlayerReference`))) (.y (`Actor.K2_GetActorLocation` (`self.PlayerReference`)))))) (`self.UnitsPerMeter`)))))
  (return))

(fn `UpdateMarkerElevations`
  (bind _defaultelevationrange (`self.DefaultElevationRange`))
  (bind _z (.z (`Actor.K2_GetActorLocation` (`self.PlayerReference`))))
  (for (_array_element _array_index) (`/Game/RadarSystem/Widgets/W_Radar.MarkerWidgets` (`self.RadarWidgetReference`))
    (bind _z_2 (.z (`.Location_5_DE6DBAFE464D624CFBEFE59C7B88E7BD` (break `/Game/RadarSystem/Structures/S_MarkerInfo` (`|GetArrayItem` (`self.QuestMarkers`) _array_index)))))
    (if (> _z_2 (+ _z _defaultelevationrange))
      (`/Game/RadarSystem/Widgets/W_Marker.SetArrowDirection` _array_element true)
      (bind _arrowimage (`/Game/RadarSystem/Widgets/W_Marker.ArrowImage` _array_element))
      (`Widget.SetVisibility` _arrowimage "SelfHitTestInvisible")
      (elif (< _z_2 (- _z _defaultelevationrange))
        (`/Game/RadarSystem/Widgets/W_Marker.SetArrowDirection` _array_element false)
        (`Widget.SetVisibility` _arrowimage "SelfHitTestInvisible")
        (else
          (`Widget.SetVisibility` _arrowimage "Hidden")))))
  (return))

(fn `UpdateMarkerPositionForMonster`
  (params (Monster :type "/Game/RadarSystem/Classes/Bp_Master_Monster Object Reference"))
  (locals (localIndex :type Integer :default 0))
  (bind _returnvalue (`KismetArrayLibrary.Array_Find` (`self.MonstersOnRadar`) Monster))
  (bind _output (`|GetArrayItem` (`/Game/RadarSystem/Widgets/W_Radar.MonsterMarkerWidgets` (`self.RadarWidgetReference`)) (`local.localIndex`)))
  (bind (_translation _clockwise_ _inradarsight_) (`self.RotationsToTranslation` (`SceneComponent.K2_GetComponentRotation` (`self.CameraReference`)) (`KismetMathLibrary.FindLookAtRotation` (`Actor.K2_GetActorLocation` (`self.PlayerReference`)) (`Actor.K2_GetActorLocation` Monster))))
  (bind _returnvalue_2 (`Widget.IsVisible` _output))
  (if (>= _returnvalue 0)
    (set `local.localIndex` _returnvalue)
    (`/Engine/EditorBlueprintResources/StandardMacros.IsValid` _output
      (:`Is Valid`
        (if _inradarsight_
          (`Widget.SetRenderTranslation` _output _translation)
          (if (not _returnvalue_2)
            (`Widget.SetVisibility` _output "SelfHitTestInvisible"))
          (elif _returnvalue_2
            (`Widget.SetVisibility` _output "Hidden")))))))

(fn `UpdateMarkerPositions`
  (bind _maxwidgettranslation (`self.MaxWidgetTranslation`))
  (for (_array_element _array_index) (`/Game/RadarSystem/Widgets/W_Radar.MarkerWidgets` (`self.RadarWidgetReference`))
    (if (`self.HideOutOfSightMarkers?`)
      (bind (_translation _clockwise_ _inradarsight_) (`self.RotationsToTranslation` (`SceneComponent.K2_GetComponentRotation` (`self.CameraReference`)) (`KismetMathLibrary.FindLookAtRotation` (`Actor.K2_GetActorLocation` (`self.PlayerReference`)) (`.Location_5_DE6DBAFE464D624CFBEFE59C7B88E7BD` (break `/Game/RadarSystem/Structures/S_MarkerInfo` (`|GetArrayItem` (`self.QuestMarkers`) _array_index))))))
      (if _inradarsight_
        (`Widget.SetRenderTranslation` _array_element _translation)
        (bind _returnvalue (`Widget.IsVisible` _array_element))
        (if (not _returnvalue)
          (`Widget.SetVisibility` _array_element "SelfHitTestInvisible"))
        (elif _returnvalue
          (`Widget.SetVisibility` _array_element "Hidden")))
      (else
        (`Widget.SetRenderTranslation` _array_element (select `bool` _inradarsight_ :`false` (`KismetMathLibrary.MakeVector2D` (`KismetMathLibrary.SelectFloat` _maxwidgettranslation (* -1 _maxwidgettranslation) _clockwise_)) :`true` _translation)))))
  (return))

(fn `UpdateMonsterMarkerDistances`
  (for _array_element (`self.MonstersOnRadar`)
    (`self.UpdateMarkerDistanceForMonster` _array_element)))

(fn `UpdateMonsterMarkerPositions`
  (for _array_element (`self.MonstersOnRadar`)
    (`self.UpdateMarkerPositionForMonster` _array_element)))