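; Base monster pawn that patrols randomly around its spawn point and reports itself to a nearby actor's radar component.
; AIMoveTo sends it to random reachable points within PatrolRadius, pausing briefly between successful moves.
; A sphere overlap adds or removes it from the radar, with an initial overlap scan on radar initialization.
; While moving on radar, a looping timer pushes position updates, cleared when it stops or leaves.
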(event `self.ReceiveBeginPlay`
  (set `self.StartLocation` (`self.K2_GetActorLocation`))
  (`self.StartPatrolling`))

(event `StartPatrolling`
  (`self.OnStartMoving`)
  (`|AIMoveTo` self (`NavigationSystem.K2_GetRandomReachablePointInRadius` (`self.StartLocation`) (`self.PatrolRadius`))
    (:`OnSuccess`
      (`self.OnStopMoving`)
      (`KismetSystemLibrary.Delay` (`KismetMathLibrary.RandomFloatInRange` 1.0 3.0))
      (`self.StartPatrolling`))))

(event `OnStartMoving`
  (set `self.CurrentlyMoving?` true)
  (if (`self.OnRadar?`)
    (`/Engine/EditorBlueprintResources/StandardMacros.IsValid` (`self.PlayerRadar`)
      (:`Is Valid`
        (`self.UpdateOnRadar`)
        (`self.StartUpdateTimer`)))))

(event `OnRadarIntialized`
  (for _array_element (`PrimitiveComponent.GetOverlappingActors` (`self.OnRadarSphere`) "/Script/Engine.Pawn")
    (bind _returnvalue (`self.GetComponentByClass` _array_element "/Game/RadarSystem/Components/BpC_RadarComponent.BpC_RadarComponent_C"))
    (`/Engine/EditorBlueprintResources/StandardMacros.IsValid` _returnvalue
      (:`Is Valid`
        (bind _success_ (`/Game/RadarSystem/Components/BpC_RadarComponent.AddMonsterToRadar` _returnvalue self))
        (if _success_
          (set `self.OnRadar?` true)
          (set `self.PlayerRadar` _returnvalue)
          (break))))))

(event `StartUpdateTimer`
  (bind _returnvalue (`KismetSystemLibrary.K2_SetTimerDelegate` (delegate `UpdateOnRadar`) (`self.RadarUpdateInterval`) true))
  (set `self.UpdateRadarTimer` _returnvalue))

(event `OnStopMoving`
  (set `self.CurrentlyMoving?` false)
  (`KismetSystemLibrary.K2_ClearAndInvalidateTimerHandle` (`self.UpdateRadarTimer`))
  (if (`self.OnRadar?`)
    (`/Engine/EditorBlueprintResources/StandardMacros.IsValid` (`self.PlayerRadar`)
      (:`Is Valid`
        (`self.UpdateOnRadar`)))))

(event `UpdateOnRadar`
  (`/Game/RadarSystem/Components/BpC_RadarComponent.OnMonsterMoved` (`self.PlayerRadar`) self))

(event `self.OnRadarSphere.OnComponentBeginOverlap`
  (params (OverlappedComponent :type "PrimitiveComponent Object Reference") (OtherActor :type "Actor Object Reference") (OtherComp :type "PrimitiveComponent Object Reference") (OtherBodyIndex :type Integer) (bFromSweep :type Boolean) (SweepResult :type "HitResult Structure (by ref)"))
  (bind _returnvalue (`self.GetComponentByClass` OtherActor "/Game/RadarSystem/Components/BpC_RadarComponent.BpC_RadarComponent_C"))
  (if (not (`self.OnRadar?`))
    (`/Engine/EditorBlueprintResources/StandardMacros.IsValid` _returnvalue
      (:`Is Valid`
        (bind _success_ (`/Game/RadarSystem/Components/BpC_RadarComponent.AddMonsterToRadar` _returnvalue self))
        (if _success_
          (set `self.OnRadar?` true)
          (set `self.PlayerRadar` _returnvalue)
          (if (`self.CurrentlyMoving?`)
            (`self.StartUpdateTimer`)))))))

(event `self.OnRadarSphere.OnComponentEndOverlap`
  (params (OverlappedComponent :type "PrimitiveComponent Object Reference") (OtherActor :type "Actor Object Reference") (OtherComp :type "PrimitiveComponent Object Reference") (OtherBodyIndex :type Integer))
  (bind _returnvalue (`self.GetComponentByClass` OtherActor "/Game/RadarSystem/Components/BpC_RadarComponent.BpC_RadarComponent_C"))
  (if (`self.OnRadar?`)
    (`/Engine/EditorBlueprintResources/StandardMacros.IsValid` _returnvalue
      (:`Is Valid`
        (set `self.OnRadar?` false)
        (`KismetSystemLibrary.K2_ClearAndInvalidateTimerHandle` (`self.UpdateRadarTimer`))
        (`/Game/RadarSystem/Components/BpC_RadarComponent.RemoveMonsterFromRadar` _returnvalue self)
        (set `self.PlayerRadar` null)))))

(fn `UserConstructionScript`
  (`SphereComponent.SetSphereRadius` (`self.PatrolSphere`) (`self.PatrolRadius`) false)
  (set `CharacterMovementComponent.MaxWalkSpeed` (`self.MovementSpeed`) (`self.CharacterMovement`))
  (`SphereComponent.SetSphereRadius` (`self.OnRadarSphere`) (`self.OnRadarRadius`) false))